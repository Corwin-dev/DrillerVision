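; Component that manages the terrain scanner's charge, shown on a viewport timer bar, with charging, humming and burst sounds.
; Scanner press and release events from the character start and stop charging; ticking raises charge along a capped arctangent power curve from the previous level, then drains it linearly, stopping at zero.
; Charge level drives charging and burst pitch, while the UserEnabled save setting gates the bar and sound playback.
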(event Custom|OnCoreVarsPassed
  (EventDispatchers|AssignOnTerrainScannerPressed (Variables|Default|GetCharacter) (delegate Custom|OnTerrainScannerPressed))
  (EventDispatchers|AssignOnTerrainScannerReleased (Variables|Default|GetCharacter) (delegate Custom|OnTerrainScannerReleased))
  (Variables|Default|SetTimer%20Bar (Variables|/Game/DrillerVision/UI/WBP_TimerBar.WBP_TimerBar_C|GetTimerBar (Variables|Default|GetWBP_TimerBar))))

(event Custom|OnTerrainScannerReleased
  (Variables|Default|SetCharging false)
  (CallFunction|ToggleChargingSound false true)
  (CallFunction|PlayBurstSound)
  (CallFunction|ToggleHummingSound true false))

(event Custom|OnTerrainScannerPressed
  (CallFunction|StartCharging)
  (CallFunction|EnableChargeBar)
  (CallFunction|ToggleChargingSound true false)
  (CallFunction|ToggleHummingSound false true))

(event EventBeginPlay
  (CallFunction|TimerBarSetup))

(event EventTick
  (params (DeltaSeconds :type Float%20%28single-precision%29))
  (CallFunction|TimerTick DeltaSeconds)
  (CallFunction|AttenuatePitch))

(fn TimerBarSetup
  (bind _returnvalue (UserInterface|CreateWidget "/Game/DrillerVision/UI/WBP_TimerBar.WBP_TimerBar_C"))
  (bind _output_get (Variables|Default|SetWBP_TimerBar _returnvalue))
  (Variables|Default|SetTimer%20Bar (Variables|/Game/DrillerVision/UI/WBP_TimerBar.WBP_TimerBar_C|GetTimerBar _output_get))
  (UserInterface|Viewport|AddtoViewport _returnvalue -1))

(fn StartCharging
  (Variables|Default|SetPrevious%20Charge (Variables|Default|GetDisplay%20Time))
  (Variables|Default|SetCharge%20Time 0.0)
  (Variables|Default|SetCharging true)
  (Components|Tick|SetComponentTickEnabled true))

(fn TimerTick
  (params (Delta :type Float%20%28single-precision%29))
  (if (Variables|Default|GetCharging)
    (bind _output_get (Variables|Default|SetCharge%20Time (+ Delta (Variables|Default|GetCharge%20Time))))
    (Variables|Default|SetDisplay%20Time (CallFunction|CalculateDisplayTime _output_get (Variables|Default|GetPrevious%20Charge)))
    (else
      (Variables|Default|SetDisplay%20Time (Math|Float|Max(Float) (- (Variables|Default|GetDisplay%20Time) Delta) 0.0))))
  (Progress|SetPercent (Variables|Default|GetTimer%20Bar) (/ (Variables|Default|GetDisplay%20Time) 24.5))
  (if (<= (Variables|Default|GetDisplay%20Time) 0.0)
    (CallFunction|StopTick)))

(fn StopTick
  (Widget|SetRenderOpacity (Variables|Default|GetWBP_TimerBar) 0.0)
  (Variables|Default|SetCharge%20Time 0.0)
  (Components|Tick|SetComponentTickEnabled false))

(fn ToggleChargeBar
  (bind _wbp_timerbar (Variables|Default|GetWBP_TimerBar))
  (if (and (> (Variables|Default|GetDisplay%20Time) 0.0) (Variables|/Game/DrillerVision/UI/SG_DrillerVision_SaveGame.SG_DrillerVision_SaveGame_C|GetUserEnabled (Variables|Default|GetSave%20Game)))
    (Widget|SetRenderOpacity _wbp_timerbar 0.5)
    (else
      (Widget|SetRenderOpacity _wbp_timerbar 0.0))))

(fn LoadReferences
  (params (SaveGame :type SG%20Driller%20Vision%20Save%20Game%20Object%20Reference%20%28by%20ref%29) (Inventory :type Inventory%20Component%20Object%20Reference%20%28by%20ref%29) (Character :type Player%20Character%20Object%20Reference%20%28by%20ref%29) (Charging%20SFX :type Audio%20Component%20Object%20Reference) (Humming%20SFX :type Audio%20Component%20Object%20Reference))
  (Variables|Default|SetSave%20Game SaveGame)
  (Variables|Default|SetInventory Inventory)
  (Variables|Default|SetCharacter Character)
  (Variables|Default|SetCharging%20SFX Charging%20SFX)
  (Variables|Default|SetHumming%20SFX Humming%20SFX)
  (CallFunction|OnCoreVarsPassed))

(fn GetDisplayTime
  (return (Variables|Default|GetDisplay%20Time)))

(fn PlayBurstSound
  (if (Variables|/Game/DrillerVision/UI/SG_DrillerVision_SaveGame.SG_DrillerVision_SaveGame_C|GetUserEnabled (Variables|Default|GetSave%20Game))
    (Audio|SpawnSoundAttached "/Game/DrillerVision/SFX/SFX_Shockwave.SFX_Shockwave" (Variables|/Script/FSD.TerrainScannerItem|GetTerrainScannerRoot (Variables|/Script/FSD.InventoryComponent|GetTerrainScannerItem (Variables|Default|GetInventory))) "None" "0, 0, 0" "0, 0, 0" "KeepRelativeOffset" false (Variables|Default|GetVolume) (- 1.0 (Variables|/Script/UMG.ProgressBar|GetPercent (Variables|Default|GetTimer%20Bar))) 0.7 0 0)))

(fn EnableChargeBar
  (if (Variables|/Game/DrillerVision/UI/SG_DrillerVision_SaveGame.SG_DrillerVision_SaveGame_C|GetUserEnabled (Variables|Default|GetSave%20Game))
    (Widget|SetRenderOpacity (Variables|Default|GetWBP_TimerBar) 0.5)))

(fn CalculateDisplayTime
  (params (Charge%20Time :type Float%20%28single-precision%29) (Previous%20Charge :type Float%20%28single-precision%29))
  (bind _returnvalue (Math|Float|Max(Float) Previous%20Charge 0.0))
  (return (Math|Float|Min(Float) (Math|Float|Max(Float) (+ (* (Math|Float|Power (Math|Trig|Atan(Degrees) (Math|Float|Max(Float) Charge%20Time 0.0)) 3.14159) (- 6.28318 (/ _returnvalue 3.9))) _returnvalue) 0.0) 24.5)))

(fn AttenuatePitch
  (Audio|Components|Audio|SetPitchMultiplier (Variables|Default|GetCharging%20SFX) (+ (Variables|/Script/UMG.ProgressBar|GetPercent (Variables|Default|GetTimer%20Bar)) 1.0)))

(fn ToggleChargingSound
  (params (Allow%20Enable :type Boolean) (Force%20Disable :type Boolean))
  (bind _charging_sfx (Variables|Default|GetCharging%20SFX))
  (if Force%20Disable
    (Audio|Components|Audio|Stop _charging_sfx :!label _label)
    (elif (Variables|/Game/DrillerVision/UI/SG_DrillerVision_SaveGame.SG_DrillerVision_SaveGame_C|GetUserEnabled (Variables|Default|GetSave%20Game))
      (if Allow%20Enable
        (Audio|Components|Audio|Play _charging_sfx 0.0))
      (else
        (goto _label)))))

(fn ToggleHummingSound
  (params (Allow%20Enable :type Boolean) (Force%20Disable :type Boolean))
  (bind _humming_sfx (Variables|Default|GetHumming%20SFX))
  (if Force%20Disable
    (Audio|Components|Audio|Stop _humming_sfx :!label _label)
    (elif (Variables|/Game/DrillerVision/UI/SG_DrillerVision_SaveGame.SG_DrillerVision_SaveGame_C|GetUserEnabled (Variables|Default|GetSave%20Game))
      (if Allow%20Enable
        (Audio|Components|Audio|Play _humming_sfx 0.0))
      (else
        (goto _label)))))
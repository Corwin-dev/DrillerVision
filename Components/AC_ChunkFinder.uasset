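; An actor component for the player character that records the terrain chunks the player has come near.
; On BeginPlay it caches the CSG world, the owning PlayerCharacter and its first-person camera.
; Every tick it queries the world for terrain actors in a fixed range around the camera and adds them to a DiscoveredChunks set.
; GetDiscoveredChunks returns that accumulated set as an array.
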(event EventBeginPlay
  (Variables|Default|SetWorld (Class|GameFunctionLibrary|GetCSGWorld))
  (bind _asplayer_character (Utilities|Casting|CastToPlayerCharacter (Components|GetOwner)))
  (bind _output_get (Variables|Default|SetPlayer _asplayer_character))
  (Variables|Default|SetFirst%20Person%20Camera (Variables|/Script/FSD.PlayerCharacter|GetFirstPersonCamera _output_get)))

(event EventTick
  (params (DeltaSeconds :type Float%20%28single-precision%29))
  (bind _terrainactors (Class|DeepCSGWorld|GetAllTerrainActorsAroundPoint (Variables|Default|GetWorld) (Transformation|GetWorldLocation (Variables|Default|GetFirst%20Person%20Camera)) (Math|Vector|MakeVector 1e+03 1e+03 1e+03)))
  (Utilities|Set|AddItems (Variables|Default|GetDiscovered%20Chunks) _terrainactors))

(fn GetDiscoveredChunks
  (bind _result (Utilities|Set|ToArray (Variables|Default|GetDiscovered%20Chunks)))
  (return _result))